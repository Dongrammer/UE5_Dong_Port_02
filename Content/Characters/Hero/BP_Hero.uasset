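; BP_Hero is the hero character Blueprint, which shows the WB_Sup HUD widget and provides keys for changing the time multiplier.
; BeginPlay creates the widget, Tick feeds it GlobalTime, and B and N call SetTimeMult for fast or slower rates.
; Tick also sweeps the character a tiny step out and back each frame.
; Montage, sphere-trace, force and InteractionCapsule overlap-binding experiments remain disconnected and never run.
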(event Custom|커스텀이벤트
  (params (OverlappedComponent :type Primitive%20Component%20Object%20Reference) (OtherActor :type Actor%20Object%20Reference) (OtherComp :type Primitive%20Component%20Object%20Reference) (OtherBodyIndex :type Integer) (bFromSweep :type Boolean) (SweepResult :type Hit%20Result%20Structure%20%28by%20ref%29))
  (Development|PrintString "Hello"))

(event EventBeginPlay
  (bind _returnvalue (UserInterface|CreateWidget "/Game/Characters/Hero/WB_Sup.WB_Sup_C"))
  (bind _output_get (Variables|Default|SetNewVar _returnvalue))
  (UserInterface|Viewport|AddtoViewport _output_get 0))

(event Collision|EventActorBeginOverlap
  (params (OtherActor :type Actor%20Object%20Reference)))

(event EventTick
  (params (DeltaSeconds :type Float%20%28single-precision%29))
  (bind _returnvalue (Transformation|GetActorRotation))
  (bind _charactermovement (Variables|Character|GetCharacterMovement))
  (bind _output_get (Variables|Default|SetGlobal%20Time (Variables|Default|GetGlobalTime)))
  (Default|SetTime (Variables|Default|GetNewVar) _output_get)
  (Class|MovementComponent|MoveUpdatedComponent _charactermovement "0.100000,0.100000,0.000000" _returnvalue true)
  (Class|MovementComponent|MoveUpdatedComponent _charactermovement "-0.100000,-0.100000,0.000000" _returnvalue true))

(event Input|KeyboardEvents|B
  (params (Key :type Key%20Structure :default "None"))
  (:Pressed
    (Class|Hero|SetTimeMult 5e+01)))

(event Input|KeyboardEvents|N
  (params (Key :type Key%20Structure :default "None"))
  (:Pressed
    (Class|Hero|SetTimeMult 2.0)))

(fn ConstructionScript)