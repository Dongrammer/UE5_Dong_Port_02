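; Dash action Blueprint that moves its ActionOwner forward, back, left or right by DashDistance.
; DoDashMovement switches on Direction, captures the start location and derives the end from the owner's forward or right vector.
; Each direction plays its own timeline, whose track drives a lerp between those points.
; Every update converts the remaining world delta to local space and applies it as a swept offset, so collision can block the dash.
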(event EventBeginPlay)

(event Collision|EventActorBeginOverlap
  (params (OtherActor :type Actor%20Object%20Reference)))

(event EventTick
  (params (DeltaSeconds :type Float%20%28single-precision%29)))

(event EventDoDashMovement
  (switch Utilities|FlowControl|Switch|SwitchonEInputDirection (Variables|Default|Getdirection)
    (:E_Forward
      ;[1 1 1] Forward Dash
      ;;[1 1 1] Set Location
      (Variables|Default|SetStartLocation (Transformation|GetActorLocation (Variables|Default|GetActionOwner)))
      (Variables|Default|SetEndLocation (+ (Variables|Default|GetStartLocation) (* (Transformation|GetActorForwardVector (Variables|Default|GetActionOwner)) (Variables|Default|GetDashDistance))))
      (bind _새_트랙_0 (Timeline|타임라인 PlayFromStart)
        (:Update
          (Transformation|AddActorLocalOffset (Variables|Default|GetActionOwner) (Class|KismetMathLibrary|MatrixInverseTransformVector (Math|Transform|ToMatrix(Transform) (Transformation|GetActorTransform (Variables|Default|GetActionOwner))) (- (Math|Vector|Lerp(Vector) (Variables|Default|GetStartLocation) (Variables|Default|GetEndLocation) _새_트랙_0) (Transformation|GetActorLocation (Variables|Default|GetActionOwner)))) true false))))
    (:E_Right
      ;[1 1 1] Right Dash
      ;;[1 1 1] Set Location
      (Variables|Default|SetStartLocation (Transformation|GetActorLocation (Variables|Default|GetActionOwner)))
      (Variables|Default|SetEndLocation (+ (Variables|Default|GetStartLocation) (* (Transformation|GetActorRightVector (Variables|Default|GetActionOwner)) (Variables|Default|GetDashDistance))))
      (bind _새_트랙_0_2 (Timeline|타임라인_0 PlayFromStart)
        (:Update
          (Transformation|AddActorLocalOffset (Variables|Default|GetActionOwner) (Class|KismetMathLibrary|MatrixInverseTransformVector (Math|Transform|ToMatrix(Transform) (Transformation|GetActorTransform (Variables|Default|GetActionOwner))) (- (Math|Vector|Lerp(Vector) (Variables|Default|GetStartLocation) (Variables|Default|GetEndLocation) _새_트랙_0_2) (Transformation|GetActorLocation (Variables|Default|GetActionOwner)))) true false))))
    (:E_Left
      ;[1 1 1] Left Dash
      ;;[1 1 1] Set Location
      (Variables|Default|SetStartLocation (Transformation|GetActorLocation (Variables|Default|GetActionOwner)))
      (Variables|Default|SetEndLocation (- (Variables|Default|GetStartLocation) (* (Transformation|GetActorRightVector (Variables|Default|GetActionOwner)) (Variables|Default|GetDashDistance))))
      (bind _새_트랙_0_3 (Timeline|타임라인_1 PlayFromStart)
        (:Update
          (Transformation|AddActorLocalOffset (Variables|Default|GetActionOwner) (Class|KismetMathLibrary|MatrixInverseTransformVector (Math|Transform|ToMatrix(Transform) (Transformation|GetActorTransform (Variables|Default|GetActionOwner))) (- (Math|Vector|Lerp(Vector) (Variables|Default|GetStartLocation) (Variables|Default|GetEndLocation) _새_트랙_0_3) (Transformation|GetActorLocation (Variables|Default|GetActionOwner)))) true false))))
    (:E_Back
      ;[1 1 1] Back Dash
      ;;[1 1 1] Set Location
      (Variables|Default|SetStartLocation (Transformation|GetActorLocation (Variables|Default|GetActionOwner)))
      (Variables|Default|SetEndLocation (- (Variables|Default|GetStartLocation) (* (Transformation|GetActorForwardVector (Variables|Default|GetActionOwner)) (Variables|Default|GetDashDistance))))
      (bind _새_트랙_0_4 (Timeline|타임라인_2 PlayFromStart)
        (:Update
          (Transformation|AddActorLocalOffset (Variables|Default|GetActionOwner) (Class|KismetMathLibrary|MatrixInverseTransformVector (Math|Transform|ToMatrix(Transform) (Transformation|GetActorTransform (Variables|Default|GetActionOwner))) (- (Math|Vector|Lerp(Vector) (Variables|Default|GetStartLocation) (Variables|Default|GetEndLocation) _새_트랙_0_4) (Transformation|GetActorLocation (Variables|Default|GetActionOwner)))) true false))))))

(fn ConstructionScript)