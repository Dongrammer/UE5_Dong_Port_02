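; Chargeable dash action that moves the owning character forward, back, left or right, farther the longer the input is held.
; DoDashMovement pauses the charge montage and starts a looping timer, whose FlipFlop raises the distance level with growing particle bursts on alternate ticks.
; On release, it plays a directional avoid montage and a timeline sweeps the owner to the target.
; Despite its name, Charging blocks re-triggering only during the dash movement.
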(event Custom|커스텀이벤트
  (Utilities|FlowControl|FlipFlop
    (:A
      (if (Variables|Default|GetbHolding)
        ;[1 1 1] Set Distance Level
        (if (< (Variables|Default|GetDistanceLevel) (Variables|Essential|GetMaxDistanceLevel))
          (Effects|SpawnEmitteratLocation "/Game/Actions/Dash/P_ChargingDash.P_ChargingDash" (Transformation|GetActorLocation (Variables|Default|GetActionOwner)) "0, 0, 0" (Utilities|Select :Index (Variables|Default|GetDistanceLevel) :Option%200 (Math|Vector|MakeVector 0.2 0.2 0.2) :Option%201 (Math|Vector|MakeVector 0.4 0.4 0.4) :Option%202 (Math|Vector|MakeVector 0.6 0.6 0.6)))
          (Variables|Default|SetDistanceLevel (+ (Variables|Default|GetDistanceLevel) 1)))
        (else
          (Variables|Default|SetLevelDistance (Utilities|Select :Index (Variables|Default|GetDistanceLevel) :Option%200 (* (Variables|Default|GetDashDistance) 0.75) :Option%201 (* (Variables|Default|GetDashDistance) 1.25) :Option%202 (* (Variables|Default|GetDashDistance) 1.5) :Option%203 (* (Variables|Default|GetDashDistance) 2.0)) :!label _label)
          ;[1 1 1] Clear Timer
          (Variables|Default|SetCharging? true)
          (Utilities|Time|ClearandInvalidateTimerbyHandle (Variables|Default|GetCheckHoldingTimer))
          (bind _output_get (Variables|Default|Setdirection (Variables|/Script/UE5_Dong_Port_02.Hero|GetinputDirection (Variables|Default|GetActionOwner))))
          (switch Utilities|FlowControl|Switch|SwitchonEInputDirection _output_get
            (:E_Forward
              (Animation|PlayAnimMontage (Variables|Default|GetActionOwner) "/Game/Animations/Gauntlet/Dash/GA_Avoid_F_M.GA_Avoid_F_M" 1.0 "None")
              ;[1 1 1] Forward Dash
              ;;[1 1 1] Set Location
              (Variables|Default|SetStartLocation (Transformation|GetActorLocation (Variables|Default|GetActionOwner)))
              (Variables|Default|SetEndLocation (+ (Variables|Default|GetStartLocation) (* (Transformation|GetActorForwardVector (Variables|Default|GetActionOwner)) (Variables|Default|GetLevelDistance))))
              (bind _새_트랙_0 (Timeline|타임라인_7 PlayFromStart)
                (:Update
                  (Transformation|AddActorLocalOffset (Variables|Default|GetActionOwner) (Class|KismetMathLibrary|MatrixInverseTransformVector (Math|Transform|ToMatrix(Transform) (Transformation|GetActorTransform (Variables|Default|GetActionOwner))) (- (Math|Vector|Lerp(Vector) (Variables|Default|GetStartLocation) (Variables|Default|GetEndLocation) _새_트랙_0) (Transformation|GetActorLocation (Variables|Default|GetActionOwner)))) true false))
                (:Finished
                  ;[1 1 1] End Move
                  (Variables|Default|SetDistanceLevel 0 :!label _label_2)
                  (Variables|Default|SetCharging? false))))
            (:E_Right
              (Animation|PlayAnimMontage (Variables|Default|GetActionOwner) "/Game/Animations/Gauntlet/Dash/GA_Avoid_R_M.GA_Avoid_R_M" 1.0 "None")
              ;[1 1 1] Right Dash
              ;;[1 1 1] Set Location
              (Variables|Default|SetStartLocation (Transformation|GetActorLocation (Variables|Default|GetActionOwner)))
              (Variables|Default|SetEndLocation (+ (Variables|Default|GetStartLocation) (* (Transformation|GetActorRightVector (Variables|Default|GetActionOwner)) (Variables|Default|GetLevelDistance))))
              (bind _새_트랙_0_2 (Timeline|타임라인_3 PlayFromStart)
                (:Update
                  (Transformation|AddActorLocalOffset (Variables|Default|GetActionOwner) (Class|KismetMathLibrary|MatrixInverseTransformVector (Math|Transform|ToMatrix(Transform) (Transformation|GetActorTransform (Variables|Default|GetActionOwner))) (- (Math|Vector|Lerp(Vector) (Variables|Default|GetStartLocation) (Variables|Default|GetEndLocation) _새_트랙_0_2) (Transformation|GetActorLocation (Variables|Default|GetActionOwner)))) true false))
                (:Finished
                  (goto _label_2))))
            (:E_Left
              (Animation|PlayAnimMontage (Variables|Default|GetActionOwner) "/Game/Animations/Gauntlet/Dash/GA_Avoid_L_M.GA_Avoid_L_M" 1.0 "None")
              ;[1 1 1] Left Dash
              ;;[1 1 1] Set Location
              (Variables|Default|SetStartLocation (Transformation|GetActorLocation (Variables|Default|GetActionOwner)))
              (Variables|Default|SetEndLocation (- (Variables|Default|GetStartLocation) (* (Transformation|GetActorRightVector (Variables|Default|GetActionOwner)) (Variables|Default|GetLevelDistance))))
              (bind _새_트랙_0_3 (Timeline|타임라인_4 PlayFromStart)
                (:Update
                  (Transformation|AddActorLocalOffset (Variables|Default|GetActionOwner) (Class|KismetMathLibrary|MatrixInverseTransformVector (Math|Transform|ToMatrix(Transform) (Transformation|GetActorTransform (Variables|Default|GetActionOwner))) (- (Math|Vector|Lerp(Vector) (Variables|Default|GetStartLocation) (Variables|Default|GetEndLocation) _새_트랙_0_3) (Transformation|GetActorLocation (Variables|Default|GetActionOwner)))) true false))
                (:Finished
                  (goto _label_2))))
            (:E_Back
              (Animation|PlayAnimMontage (Variables|Default|GetActionOwner) "/Game/Animations/Gauntlet/Dash/GA_Avoid_B_M.GA_Avoid_B_M" 1.0 "None")
              ;[1 1 1] Back Dash
              ;;[1 1 1] Set Location
              (Variables|Default|SetStartLocation (Transformation|GetActorLocation (Variables|Default|GetActionOwner)))
              (Variables|Default|SetEndLocation (- (Variables|Default|GetStartLocation) (* (Transformation|GetActorForwardVector (Variables|Default|GetActionOwner)) (Variables|Default|GetLevelDistance))))
              (bind _새_트랙_0_4 (Timeline|타임라인_5 PlayFromStart)
                (:Update
                  (Transformation|AddActorLocalOffset (Variables|Default|GetActionOwner) (Class|KismetMathLibrary|MatrixInverseTransformVector (Math|Transform|ToMatrix(Transform) (Transformation|GetActorTransform (Variables|Default|GetActionOwner))) (- (Math|Vector|Lerp(Vector) (Variables|Default|GetStartLocation) (Variables|Default|GetEndLocation) _새_트랙_0_4) (Transformation|GetActorLocation (Variables|Default|GetActionOwner)))) true false))
                (:Finished
                  (goto _label_2))))))))
    (:B
      (if (not (Variables|Default|GetbHolding)) ; Button Released
        (goto _label)))))

(event EventBeginPlay)

(event Collision|EventActorBeginOverlap
  (params (OtherActor :type Actor%20Object%20Reference)))

(event EventTick
  (params (DeltaSeconds :type Float%20%28single-precision%29)))

(event EventDoDashMovement
  (if (not (Variables|Default|GetCharging?))
    (Class|AnimInstance|MontagePause (Components|SkeletalMesh|GetAnimInstance (Variables|/Script/Engine.Character|GetMesh (Variables|Default|GetActionOwner))) "/Game/Animations/Gauntlet/Dash/GA_ChargingAvoid_M.GA_ChargingAvoid_M")
    (bind _returnvalue (Utilities|Time|SetTimerbyEvent (delegate Custom|커스텀이벤트) 0.2 true))
    (Variables|Default|SetCheckHoldingTimer _returnvalue)))

(fn ConstructionScript)