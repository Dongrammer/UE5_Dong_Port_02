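; BP_Act_GA_Kick_01 is a kick action actor that moves its ActionOwner during the attack.
; DoActionMovement calls SetLocation, then plays a timeline whose Move curve lerps between StartLocation and EndLocation.
; Each update applies the step as a swept local offset through an inverse transform and stops the timeline once the owner leaves EAttack.
; An inline forward-by-MoveDistance endpoint calculation remains in the graph but never runs.
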(event EventBeginPlay)

(event Collision|EventActorBeginOverlap
  (params (OtherActor :type Actor%20Object%20Reference)))

(event EventTick
  (params (DeltaSeconds :type Float%20%28single-precision%29)))

(event EventDoActionMovement
  (bind _actionowner (Variables|Default|GetActionOwner))
  (Class|BaseAction|SetLocation)
  (bind _move (Timeline|타임라인 PlayFromStart)
    (:Update
      (Transformation|AddActorLocalOffset _actionowner (Class|KismetMathLibrary|MatrixInverseTransformVector (Math|Transform|ToMatrix(Transform) (Transformation|GetActorTransform _actionowner)) (- (Math|Vector|Lerp(Vector) (Variables|Default|GetStartLocation) (Variables|Default|GetEndLocation) _move) (Transformation|GetActorLocation (Variables|Default|GetActionOwner)))) true false)
      (bind _returnvalue (Class|Hero|CurrentStateIs (Variables|Default|GetActionOwner) "E_Attack"))
      (if (not _returnvalue)
        (Timeline|타임라인 Stop)))))

(fn ConstructionScript)